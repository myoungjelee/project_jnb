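; BP_TutorialPortal is a portal actor that loads the tutorial level when Enter is pressed inside its overlap area.
; It creates a BP_TextTuto widget at BeginPlay, then shows it with a sound on overlap and removes it on exit.
; Overlap also enables input and sets the On flag that gates the level load; neither overlap event checks which actor triggered it.
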(event EventBeginPlay
  (bind _returnvalue (UserInterface|CreateWidget "/Game/Blueprints/BP_TextTuto.BP_TextTuto_C"))
  (Variables|Default|SetEnter _returnvalue))

(event Collision|EventActorBeginOverlap
  (params (OtherActor :type Actor%20Object%20Reference))
  (UserInterface|Viewport|AddtoViewport (Variables|Default|GetEnter) 0)
  (Variables|Default|SetOn true)
  (Audio|PlaySound2D "/Game/Audio/Exit.Exit" 1.0 1.0 0.0 0 0)
  (Input|EnableInput (Game|GetPlayerController 0)))

(event EventTick
  (params (DeltaSeconds :type Float%20%28single-precision%29)))

(event Collision|EventActorEndOverlap
  (params (OtherActor :type Actor%20Object%20Reference))
  (Widget|RemovefromParent (Variables|Default|GetEnter))
  (Variables|Default|SetOn false))

(event Input|KeyboardEvents|Enter
  (params (Key :type Key%20Structure :default "None"))
  (:Pressed
    (if (Variables|Default|GetOn)
      (Game|OpenLevel(byObjectReference) "/Game/Levels/TutorialLevel.TutorialLevel"))))

(fn ConstructionScript)