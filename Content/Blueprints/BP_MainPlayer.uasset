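; BP_MainPlayer is the player Blueprint that manages background music, the in-game UI, pause and game over.
; BeginPlay starts the BGM as a 2D sound and adds the game UI widget to the viewport.
; Tab flips a Paused flag to toggle game pause, music pause and the pause widget, showing the cursor on pause.
; Destruction serves as game over, pausing the game, stopping music and swapping the UI for a game-over widget.
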(event EventDestroyed
  (Game|SetGamePaused true)
  (Audio|Components|Audio|Stop (Variables|Default|GetBGM))
  (Variables|/Script/Engine.PlayerController|SetbShowMouseCursor (Game|GetPlayerController 0) true)
  (bind _returnvalue (UserInterface|CreateWidget "/Game/Blueprints/BP_GameOverWidget.BP_GameOverWidget_C"))
  (UserInterface|Viewport|AddtoViewport _returnvalue 0)
  (Widget|RemovefromParent (Variables|Default|GetGameUI)))

(event EventBeginPlay
  (bind _returnvalue (Audio|SpawnSound2D "/Game/Audio/BGM.BGM" 1.0 1.0 0.0 0))
  (Variables|Default|SetBGM _returnvalue)
  (bind _returnvalue_2 (UserInterface|CreateWidget "/Game/Blueprints/BP_GameUI.BP_GameUI_C"))
  (bind _output_get (Variables|Default|SetGameUI _returnvalue_2))
  (UserInterface|Viewport|AddtoViewport _output_get 0))

(event EventTick
  (params (DeltaSeconds :type Float%20%28single-precision%29)))

(event Input|KeyboardEvents|Tab
  (params (Key :type Key%20Structure :default "None"))
  (:Pressed
    (if (Variables|Default|GetbPaused)
      (Variables|Default|SetbPaused false)
      (Game|SetGamePaused false)
      (Class|AudioComponent|SetPaused (Variables|Default|GetBGM) false)
      (Widget|RemovefromParent (Variables|Default|GetPause))
      (else
        (Variables|Default|SetbPaused true)
        (Game|SetGamePaused true)
        (Class|AudioComponent|SetPaused (Variables|Default|GetBGM) true)
        (Variables|/Script/Engine.PlayerController|SetbShowMouseCursor (Game|GetPlayerController 0) true)
        (bind _returnvalue (UserInterface|CreateWidget "/Game/Blueprints/BP_PauseWidget.BP_PauseWidget_C"))
        (bind _output_get (Variables|Default|SetPause _returnvalue))
        (UserInterface|Viewport|AddtoViewport _output_get 0)))))

(fn ConstructionScript)