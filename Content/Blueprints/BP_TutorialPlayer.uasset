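; BP_TutorialPlayer is the tutorial player Blueprint, handling the HUD, background music and pause menu.
; On BeginPlay it adds the BP_GameUI_2 widget to the viewport and starts the tutorial music, keeping it as BGM.
; Tab toggles game and music pause along with the BP_PauseTuto widget.
; Pausing shows the mouse cursor, but unpausing does not hide it again.
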(event EventDestroyed)

(event EventBeginPlay
  (bind _returnvalue (UserInterface|CreateWidget "/Game/Blueprints/BP_GameUI_2.BP_GameUI_2_C"))
  (UserInterface|Viewport|AddtoViewport _returnvalue 0)
  (bind _returnvalue_2 (Audio|SpawnSound2D "/Game/Audio/Tutotial.Tutotial" 1.0 1.0 0.0 0))
  (Variables|Default|SetBGM _returnvalue_2))

(event EventTick
  (params (DeltaSeconds :type Float%20%28single-precision%29)))

(event Input|KeyboardEvents|Tab
  (params (Key :type Key%20Structure))
  (:Pressed
    (if (Variables|Default|GetbPaused)
      (Variables|Default|SetbPaused false)
      (Game|SetGamePaused false)
      (Class|AudioComponent|SetPaused (Variables|Default|GetBGM) false)
      (Widget|RemovefromParent (stale _returnvalue))
      (else
        (Variables|Default|SetbPaused true)
        (Game|SetGamePaused true)
        (Class|AudioComponent|SetPaused (Variables|Default|GetBGM) true)
        (Variables|/Script/Engine.PlayerController|SetbShowMouseCursor (Game|GetPlayerController 0) true)
        (bind _returnvalue (UserInterface|CreateWidget "/Game/Blueprints/BP_PauseTuto.BP_PauseTuto_C"))
        (UserInterface|Viewport|AddtoViewport _returnvalue 0)))))

(fn ConstructionScript)